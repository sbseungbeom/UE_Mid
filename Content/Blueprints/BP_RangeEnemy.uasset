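; BP_RangeEnemy is an enemy that approaches its Target, with ranged attacking still unimplemented as Shoot is empty.
; Tick moves it toward Target by local offset from a world-space direction until any Sphere overlap permanently clears CanTrackPlayer, then it only rotates to face Target.
; Any Box overlap runs DieProcess, spawning a huge Niagara explosion and destroying the actor only if Target casts to BP_P.
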(event `self.ReceiveBeginPlay`)

(event `self.ReceiveTick`
  (params (DeltaSeconds :type "Float (single-precision)"))
  (if (`self.canTrackPlayer`)
    (bind _output_get (set `self.DirVector` (- (`self.K2_GetActorLocation` (`self.Target`)) (`self.K2_GetActorLocation`))))
    (`self.K2_AddActorLocalOffset` (* (`KismetMathLibrary.Normal` _output_get) (`self.MoveSpeed`) DeltaSeconds))
    (else
      (`self.K2_SetActorRotation` (`KismetMathLibrary.FindLookAtRotation` (`self.K2_GetActorLocation`) (`self.K2_GetActorLocation` (`self.Target`)))))))

(event `self.Sphere.OnComponentBeginOverlap`
  (params (OverlappedComponent :type "PrimitiveComponent Object Reference") (OtherActor :type "Actor Object Reference") (OtherComp :type "PrimitiveComponent Object Reference") (OtherBodyIndex :type Integer) (bFromSweep :type Boolean) (SweepResult :type "HitResult Structure (by ref)"))
  (set `self.canTrackPlayer` false))

(event `self.Box.OnComponentBeginOverlap`
  (params (OverlappedComponent :type "PrimitiveComponent Object Reference") (OtherActor :type "Actor Object Reference") (OtherComp :type "PrimitiveComponent Object Reference") (OtherBodyIndex :type Integer) (bFromSweep :type Boolean) (SweepResult :type "HitResult Structure (by ref)"))
  (`self.DieProcess`))

(fn `DieProcess`
  (`NiagaraFunctionLibrary.SpawnSystemAtLocation` "/Game/Assets/Fire_EXP_Vol01_Free/Niagara/EXP/NS_Sub_EXP_Large_001_01.NS_Sub_EXP_Large_001_01" (`self.K2_GetActorLocation`) (struct) (1000.0 1000.0 1000.0))
  (cast `/Game/Blueprints/BP_P` (`self.Target`))
  (`self.K2_DestroyActor`))

(fn `Shoot`)

(fn `UserConstructionScript`)