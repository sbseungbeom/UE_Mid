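; BP_EnemySpawner is an actor that periodically spawns BP_Enemy instances of its configured EnemyType, targeting the player.
; Tick accumulates time until SpawnTimer, then SpawnEnemy spawns at the spawner's location, configures by type and resets the timer.
; Normal adds a second, offset enemy.
; Straight moves along negative X, while Kamikaze moves faster toward the player's position at spawn, both with tracking disabled.
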(event `self.ReceiveBeginPlay`)

(event `self.ReceiveTick`
  (params (DeltaSeconds :type "Float (single-precision)"))
  (bind _output_get (set `self.CurrnetTime` (+ DeltaSeconds (`self.CurrnetTime`))))
  (if (>= _output_get (`self.SpawnTimer`))
    (`self.SpawnEnemy` (`self.EnemyType`))))

(fn `SpawnEnemy`
  (params (EnemyType :type "/Game/Blueprints/Enemy/Enum_EnemyType Enum" :default "NewEnumerator0"))
  (locals (Enemy :type "/Game/Blueprints/BP_Enemy Object Reference"))
  (bind _enemy (`local.Enemy`))
  (bind _enemy_2 (`local.Enemy`))
  (bind _returnvalue (`|SpawnActorFromClass` "/Game/Blueprints/BP_Enemy.BP_Enemy_C" (`KismetMathLibrary.MakeTransform` (`self.K2_GetActorLocation`)) "AdjustIfPossibleButDontSpawnIfColliding" "MultiplyWithRoot" null null))
  (bind _asbp_enemy (cast `/Game/Blueprints/BP_Enemy` _returnvalue))
  (set `local.Enemy` _asbp_enemy)
  (set `/Game/Blueprints/BP_Enemy.Target` (`self.Player`) _asbp_enemy)
  (set `/Game/Blueprints/BP_Enemy.Type` EnemyType _asbp_enemy)
  (switch `/Game/Blueprints/Enemy/Enum_EnemyType` EnemyType
    (:`NewEnumerator0`
      ; 기본 스폰과 동일
      (bind _returnvalue_2 (`|SpawnActorFromClass` "/Game/Blueprints/BP_Enemy.BP_Enemy_C" (`KismetMathLibrary.MakeTransform` (+ (`self.K2_GetActorLocation`) (2000.0 2000.0 0.0))) "AdjustIfPossibleButDontSpawnIfColliding" "MultiplyWithRoot" null null))
      (bind _asbp_enemy_2 (cast `/Game/Blueprints/BP_Enemy` _returnvalue_2))
      (set `local.Enemy` _asbp_enemy_2)
      (set `/Game/Blueprints/BP_Enemy.Target` (`self.Player`) _asbp_enemy_2)
      (set `/Game/Blueprints/BP_Enemy.Type` "NewEnumerator0" _asbp_enemy_2))
    (:`NewEnumerator1`
      (set `/Game/Blueprints/BP_Enemy.DirVector` (-1.0 0.0 0.0) _enemy)
      (set `/Game/Blueprints/BP_Enemy.MoveSpeed` 10000.0 _enemy)
      (set `/Game/Blueprints/BP_Enemy.canTrackPlayer` false _enemy))
    (:`NewEnumerator4`
      (set `/Game/Blueprints/BP_Enemy.DirVector` (- (`self.K2_GetActorLocation` (`self.Player`)) (`self.K2_GetActorLocation` (`local.Enemy`))) _enemy_2)
      (set `/Game/Blueprints/BP_Enemy.MoveSpeed` 20000.0 _enemy_2)
      (set `/Game/Blueprints/BP_Enemy.canTrackPlayer` false _enemy_2)))
  (set `self.CurrnetTime` 0.0))

(fn `UserConstructionScript`)