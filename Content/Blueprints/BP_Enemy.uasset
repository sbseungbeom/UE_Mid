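; BP_Enemy is an enemy actor that chases the BP_P actor and explodes on contact.
; BeginPlay caches the BP_P as Target, and Tick moves along the normalized direction to it at MoveSpeed, applying that world-space vector as a local offset without sweep.
; Any overlap on its Box component calls DieProcess, which spawns a Niagara explosion at its location and destroys the actor.
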(event `self.ReceiveBeginPlay`
  (bind _returnvalue (`GameplayStatics.GetActorOfClass` "/Game/Blueprints/BP_P.BP_P_C"))
  (set `self.Target` _returnvalue))

(event `self.ReceiveTick`
  (params (DeltaSeconds :type "Float (single-precision)"))
  (bind _output_get (set `self.DirVector` (- (`self.K2_GetActorLocation` (`self.Target`)) (`self.K2_GetActorLocation`))))
  (`self.K2_AddActorLocalOffset` (* (`KismetMathLibrary.Normal` _output_get) (`self.MoveSpeed`) DeltaSeconds)))

(event `self.Box.OnComponentBeginOverlap`
  (params (OverlappedComponent :type "PrimitiveComponent Object Reference") (OtherActor :type "Actor Object Reference") (OtherComp :type "PrimitiveComponent Object Reference") (OtherBodyIndex :type Integer) (bFromSweep :type Boolean) (SweepResult :type "HitResult Structure (by ref)"))
  (`self.DieProcess`))

(fn `DieProcess`
  (`NiagaraFunctionLibrary.SpawnSystemAtLocation` "/Game/Assets/Fire_EXP_Vol01_Free/Niagara/EXP/NS_Sub_EXP_Large_001_01.NS_Sub_EXP_Large_001_01" (`self.K2_GetActorLocation`))
  (`self.K2_DestroyActor`))

(fn `UserConstructionScript`)