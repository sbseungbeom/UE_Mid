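; Boss enemy that, after a start delay, fires bullet-hell patterns of BP_EnemyBullet and loses health on each box overlap.
; Tick uses a CanShoot gate to pick one of three Delay-timed patterns: forward volleys, player-aimed tracking shots, or radial rings.
; The ring pattern re-enables CanShoot, then continues into tracking fire, overlapping the next pattern.
; At zero Hp it explodes, removes enemy spawners, spawns BP_GG and destroys itself, with a delayed QuitGame chained afterward.
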(event `self.ReceiveBeginPlay`
  (bind _returnvalue (`GameplayStatics.GetActorOfClass` "/Game/Blueprints/BP_P.BP_P_C"))
  (set `self.Target` _returnvalue)
  (`KismetSystemLibrary.Delay` 10.0)
  (set `self.UpdateStart` true))

(event `self.ReceiveTick`
  (params (DeltaSeconds :type "Float (single-precision)"))
  (if (<= (`self.Hp`) 0)
    (`self.DieProcess`)
    (`KismetSystemLibrary.Delay` 10.0)
    (`KismetSystemLibrary.QuitGame` null "Quit")
    (elif (`self.UpdateStart`)
      (if (`self.canShoot`)
        (set `self.canShoot` false)
        (switch `int` (`KismetMathLibrary.RandomIntegerInRange` 0 2)
          (:`0`
            ; pattern 1
            (`self.ForwardFirePattern`)
            (`KismetSystemLibrary.Delay` 0.5)
            (`self.ForwardFirePattern`)
            (`KismetSystemLibrary.Delay` 0.6)
            (`self.ForwardFirePattern`)
            (`KismetSystemLibrary.Delay` 0.7)
            (`self.ForwardFirePattern`)
            (`KismetSystemLibrary.Delay` 0.8)
            (`self.ForwardFirePattern`)
            (`KismetSystemLibrary.Delay` 0.9)
            (`self.ForwardFirePattern`)
            (`KismetSystemLibrary.Delay` 3.0)
            (set `self.canShoot` true))
          (:`1`
            ; Pattern2
            (`self.TrakingFire`)
            (`KismetSystemLibrary.Delay` 0.25)
            (`self.TrakingFire`)
            (`KismetSystemLibrary.Delay` 0.25)
            (`self.TrakingFire`)
            (`KismetSystemLibrary.Delay` 0.25)
            (`self.TrakingFire`)
            (`KismetSystemLibrary.Delay` 0.25)
            (`self.TrakingFire`)
            (`KismetSystemLibrary.Delay` 0.25)
            (`self.TrakingFire`)
            (`KismetSystemLibrary.Delay` 0.25)
            (`self.TrakingFire`)
            (`KismetSystemLibrary.Delay` 0.25)
            (`self.TrakingFire`)
            (`KismetSystemLibrary.Delay` 0.25)
            (`self.TrakingFire`)
            (`KismetSystemLibrary.Delay` 0.25)
            (`self.TrakingFire`)
            (`KismetSystemLibrary.Delay` 0.25)
            (`self.TrakingFire`)
            (`KismetSystemLibrary.Delay` 0.25)
            (`self.TrakingFire`)
            (`KismetSystemLibrary.Delay` 0.25)
            (`self.TrakingFire`)
            (`KismetSystemLibrary.Delay` 0.25)
            (`self.TrakingFire`)
            (`KismetSystemLibrary.Delay` 0.25)
            (`self.TrakingFire`)
            (`KismetSystemLibrary.Delay` 0.25)
            (`self.TrakingFire`)
            (`KismetSystemLibrary.Delay` 0.25)
            (`self.TrakingFire`)
            (`KismetSystemLibrary.Delay` 0.25)
            (`self.TrakingFire`)
            (`KismetSystemLibrary.Delay` 0.25)
            (`self.TrakingFire`)
            (`KismetSystemLibrary.Delay` 0.25)
            (`self.TrakingFire`)
            (`KismetSystemLibrary.Delay` 0.25)
            (`self.TrakingFire`)
            (`KismetSystemLibrary.Delay` 0.25)
            (`self.TrakingFire`)
            (`KismetSystemLibrary.Delay` 0.25)
            (`self.TrakingFire`)
            (`KismetSystemLibrary.Delay` 0.25)
            (`self.TrakingFire`)
            (`KismetSystemLibrary.Delay` 0.25)
            (`self.TrakingFire`)
            (`KismetSystemLibrary.Delay` 0.25)
            (`self.TrakingFire`)
            (`KismetSystemLibrary.Delay` 0.25)
            (`self.TrakingFire`)
            (`KismetSystemLibrary.Delay` 0.25)
            (`self.TrakingFire`)
            (`KismetSystemLibrary.Delay` 0.25)
            (`self.TrakingFire`)
            (`KismetSystemLibrary.Delay` 0.25)
            (`self.TrakingFire`)
            (`KismetSystemLibrary.Delay` 0.25)
            (`self.TrakingFire`)
            (`KismetSystemLibrary.Delay` 0.25)
            (`self.TrakingFire`)
            (`KismetSystemLibrary.Delay` 0.25)
            (`KismetSystemLibrary.Delay` 6.0)
            (set `self.canShoot` true))
          (:`2`
            ; Pattern3
            (`self.MidRoundFire`)
            (`KismetSystemLibrary.Delay` 1.0)
            (`self.WingRoundFire`)
            (`KismetSystemLibrary.Delay` 1.5)
            (`self.MidRoundFire`)
            (`KismetSystemLibrary.Delay` 1.0)
            (`self.WingRoundFire`)
            (`KismetSystemLibrary.Delay` 1.5)
            (`self.MidRoundFire`)
            (`KismetSystemLibrary.Delay` 3.0)
            (`self.MidRoundFire`)
            (`KismetSystemLibrary.Delay` 1.0)
            (`self.WingRoundFire`)
            (`KismetSystemLibrary.Delay` 1.5)
            (`self.MidRoundFire`)
            (`KismetSystemLibrary.Delay` 1.0)
            (`self.WingRoundFire`)
            (`KismetSystemLibrary.Delay` 1.5)
            (`self.MidRoundFire`)
            (`self.WingRoundFire`)
            (`self.MidRoundFire`)
            (`KismetSystemLibrary.Delay` 0.3)
            (`self.WingRoundFire`)
            (`self.MidRoundFire`)
            (`KismetSystemLibrary.Delay` 0.3)
            (`self.WingRoundFire`)
            (`self.MidRoundFire`)
            (`KismetSystemLibrary.Delay` 0.3)
            (`self.WingRoundFire`)
            (`self.MidRoundFire`)
            (`KismetSystemLibrary.Delay` 0.3)
            (`self.WingRoundFire`)
            (`self.MidRoundFire`)
            (`KismetSystemLibrary.Delay` 4.0)
            (set `self.canShoot` true)
            ; Pattern2
            (`self.TrakingFire`)
            (`KismetSystemLibrary.Delay` 0.25)
            (`self.TrakingFire`)
            (`KismetSystemLibrary.Delay` 0.25)
            (`self.TrakingFire`)
            (`KismetSystemLibrary.Delay` 0.25)
            (`self.TrakingFire`)
            (`KismetSystemLibrary.Delay` 0.25)
            (`self.TrakingFire`)
            (`KismetSystemLibrary.Delay` 0.25)
            (`self.TrakingFire`)
            (`KismetSystemLibrary.Delay` 0.25)
            (`self.TrakingFire`)
            (`KismetSystemLibrary.Delay` 0.25)
            (`self.TrakingFire`)
            (`KismetSystemLibrary.Delay` 0.25)
            (`self.TrakingFire`)
            (`KismetSystemLibrary.Delay` 0.25)
            (`self.TrakingFire`)
            (`KismetSystemLibrary.Delay` 0.25)
            (`self.TrakingFire`)
            (`KismetSystemLibrary.Delay` 0.25)
            (`self.TrakingFire`)
            (`KismetSystemLibrary.Delay` 0.25)
            (`self.TrakingFire`)
            (`KismetSystemLibrary.Delay` 0.25)
            (`self.TrakingFire`)
            (`KismetSystemLibrary.Delay` 0.25)
            (`self.TrakingFire`)
            (`KismetSystemLibrary.Delay` 0.25)
            (`self.TrakingFire`)
            (`KismetSystemLibrary.Delay` 0.25)
            (`self.TrakingFire`)
            (`KismetSystemLibrary.Delay` 0.25)
            (`self.TrakingFire`)
            (`KismetSystemLibrary.Delay` 0.25)
            (`self.TrakingFire`)
            (`KismetSystemLibrary.Delay` 0.25)
            (`self.TrakingFire`)
            (`KismetSystemLibrary.Delay` 0.25)
            (`self.TrakingFire`)
            (`KismetSystemLibrary.Delay` 0.25)
            (`self.TrakingFire`)
            (`KismetSystemLibrary.Delay` 0.25)
            (`self.TrakingFire`)
            (`KismetSystemLibrary.Delay` 0.25)
            (`self.TrakingFire`)
            (`KismetSystemLibrary.Delay` 0.25)
            (`self.TrakingFire`)
            (`KismetSystemLibrary.Delay` 0.25)
            (`self.TrakingFire`)
            (`KismetSystemLibrary.Delay` 0.25)
            (`self.TrakingFire`)
            (`KismetSystemLibrary.Delay` 0.25)
            (`self.TrakingFire`)
            (`KismetSystemLibrary.Delay` 0.25)
            (`self.TrakingFire`)
            (`KismetSystemLibrary.Delay` 0.25)
            (`self.TrakingFire`)
            (`KismetSystemLibrary.Delay` 0.25)
            (`self.TrakingFire`)
            (`KismetSystemLibrary.Delay` 0.25)
            (`self.TrakingFire`)
            (`KismetSystemLibrary.Delay` 0.25)))))))

(event `self.Box.OnComponentBeginOverlap`
  (params (OverlappedComponent :type "PrimitiveComponent Object Reference") (OtherActor :type "Actor Object Reference") (OtherComp :type "PrimitiveComponent Object Reference") (OtherBodyIndex :type Integer) (bFromSweep :type Boolean) (SweepResult :type "HitResult Structure (by ref)"))
  (bind _result (`/Engine/EditorBlueprintResources/StandardMacros.DecrementInt` (`self.Hp`))
    (:`  `
      (set `self.Hp` _result))))

(fn `DieProcess`
  (`NiagaraFunctionLibrary.SpawnSystemAtLocation` "/Game/Assets/Fire_EXP_Vol01_Free/Niagara/EXP/NS_Sub_EXP_Large_001_01.NS_Sub_EXP_Large_001_01" (`self.K2_GetActorLocation`) (struct) (1000.0 1000.0 1000.0))
  (bind _outactors (`GameplayStatics.GetAllActorsOfClass` "/Game/Blueprints/Enemy/BP_EnemySpawner.BP_EnemySpawner_C"))
  (for _array_element _outactors
    (`self.K2_DestroyActor` _array_element))
  (`|SpawnActorFromClass` "/Game/Assets/BP_GG.BP_GG_C" (`KismetMathLibrary.MakeTransform` (-2390.0 -5350.0 830.0)) "AlwaysSpawn" "MultiplyWithRoot" null null)
  (`GameplayStatics.PlaySound2D` "/Game/Assets/bossexp.bossexp" 1.0 1.0 0.0 null null)
  (`self.K2_DestroyActor`))

(fn `ForwardFirePattern`
  (`|ExecutionSequence`
    (:`then_0`
      (`|SpawnActorFromClass` "/Game/Blueprints/Enemy/BP_EnemyBullet.BP_EnemyBullet_C" (`KismetMathLibrary.MakeTransform` (`SceneComponent.K2_GetComponentLocation` (`self.BulletLeft`)) (struct :`Yaw` 180.0)) "AlwaysSpawn" "MultiplyWithRoot" null null))
    (:`then_1`
      (`|SpawnActorFromClass` "/Game/Blueprints/Enemy/BP_EnemyBullet.BP_EnemyBullet_C" (`KismetMathLibrary.MakeTransform` (`SceneComponent.K2_GetComponentLocation` (`self.BulletLeft1`)) (struct :`Yaw` 180.0)) "AlwaysSpawn" "MultiplyWithRoot" null null))
    (:`then_2`
      (`|SpawnActorFromClass` "/Game/Blueprints/Enemy/BP_EnemyBullet.BP_EnemyBullet_C" (`KismetMathLibrary.MakeTransform` (`SceneComponent.K2_GetComponentLocation` (`self.BulletMiddle`)) (struct :`Yaw` 180.0)) "AlwaysSpawn" "MultiplyWithRoot" null null))
    (:`then_3`
      (`|SpawnActorFromClass` "/Game/Blueprints/Enemy/BP_EnemyBullet.BP_EnemyBullet_C" (`KismetMathLibrary.MakeTransform` (`SceneComponent.K2_GetComponentLocation` (`self.BulletMiddle2`)) (struct :`Yaw` 180.0)) "AlwaysSpawn" "MultiplyWithRoot" null null))
    (:`then_4`
      (`|SpawnActorFromClass` "/Game/Blueprints/Enemy/BP_EnemyBullet.BP_EnemyBullet_C" (`KismetMathLibrary.MakeTransform` (`SceneComponent.K2_GetComponentLocation` (`self.BulletMiddle3`)) (struct :`Yaw` 180.0)) "AlwaysSpawn" "MultiplyWithRoot" null null))
    (:`then_5`
      (`|SpawnActorFromClass` "/Game/Blueprints/Enemy/BP_EnemyBullet.BP_EnemyBullet_C" (`KismetMathLibrary.MakeTransform` (`SceneComponent.K2_GetComponentLocation` (`self.BulletRIght`)) (struct :`Yaw` 180.0)) "AlwaysSpawn" "MultiplyWithRoot" null null))
    (:`then_6`
      (`|SpawnActorFromClass` "/Game/Blueprints/Enemy/BP_EnemyBullet.BP_EnemyBullet_C" (`KismetMathLibrary.MakeTransform` (`SceneComponent.K2_GetComponentLocation` (`self.BulletRIght1`)) (struct :`Yaw` 180.0)) "AlwaysSpawn" "MultiplyWithRoot" null null))))

(fn `MidRoundFire`
  (for _index (range 37)
    (`|SpawnActorFromClass` "/Game/Blueprints/Enemy/BP_EnemyBullet.BP_EnemyBullet_C" (`KismetMathLibrary.MakeTransform` (`self.K2_GetActorLocation`) (`KismetMathLibrary.MakeRotator` 0.0 0.0 (`KismetMathLibrary.Conv_IntToDouble` (* _index 10)))) "Undefined" "MultiplyWithRoot" null null)))

(fn `TrakingFire`
  (locals (PlayerPosition :type "Vector Structure") (NewLocalVar :type "Transform Structure"))
  (bind _returnvalue (`KismetMathLibrary.FindLookAtRotation` (`self.K2_GetActorLocation`) (`self.K2_GetActorLocation` (`self.Target`))))
  (`|SpawnActorFromClass` "/Game/Blueprints/Enemy/BP_EnemyBullet.BP_EnemyBullet_C" (`KismetMathLibrary.MakeTransform` (`SceneComponent.K2_GetComponentLocation` (`self.Tracker`)) _returnvalue) "AlwaysSpawn" "MultiplyWithRoot" null null)
  (`|SpawnActorFromClass` "/Game/Blueprints/Enemy/BP_EnemyBullet.BP_EnemyBullet_C" (`KismetMathLibrary.MakeTransform` (`SceneComponent.K2_GetComponentLocation` (`self.Tracker1`)) _returnvalue) "AlwaysSpawn" "MultiplyWithRoot" null null))

(fn `UserConstructionScript`)

(fn `WingRoundFire`
  (for _index (range 37)
    (bind _returnvalue (`KismetMathLibrary.Conv_IntToDouble` (* _index 10)))
    (`|SpawnActorFromClass` "/Game/Blueprints/Enemy/BP_EnemyBullet.BP_EnemyBullet_C" (`KismetMathLibrary.MakeTransform` (`SceneComponent.K2_GetComponentLocation` (`self.Tracker`)) (`KismetMathLibrary.MakeRotator` 0.0 0.0 _returnvalue)) "Undefined" "MultiplyWithRoot" null null)
    (`|SpawnActorFromClass` "/Game/Blueprints/Enemy/BP_EnemyBullet.BP_EnemyBullet_C" (`KismetMathLibrary.MakeTransform` (`SceneComponent.K2_GetComponentLocation` (`self.Tracker1`)) (`KismetMathLibrary.MakeRotator` 0.0 0.0 _returnvalue)) "Undefined" "MultiplyWithRoot" null null)))