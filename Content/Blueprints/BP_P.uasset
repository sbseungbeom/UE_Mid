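; BP_P is the player-controlled actor, which moves and automatically fires bullets.
; BeginPlay adds the player input mapping context, and both move actions share one node writing their value to X and Y of the direction, zeroed on release.
; Tick performs a swept move along that direction and spawns BP_Bullet at the Muzzle whenever the fire delay elapses.
; A Hit function destroys the actor but is not called within this Blueprint.
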(event `self.ReceiveBeginPlay`
  (`EnhancedInputSubsystemInterface.AddMappingContext` (pcsubsystem `EnhancedInputLocalPlayerSubsystem` (`GameplayStatics.GetPlayerController` 0)) "/Game/Blueprints/Inputs/IMC_Player.IMC_Player" 0 (struct)))

(event `self.ReceiveTick`
  (params (DeltaSeconds :type "Float (single-precision)"))
  (`self.Move` (`self.OrientedDirection`) (`self.MoveSpeed`))
  (bind _output_get (set `self.CurrentFireDelay` (+ DeltaSeconds (`self.CurrentFireDelay`))))
  (if (>= _output_get (`self.FireDelay`))
    (`self.Fire`)))

(event `EnhancedInput|/Game/Blueprints/Inputs/IA_MoveRight`
  (params (ActionValue :type "Float (double-precision)") (ElapsedSeconds :type "Float (double-precision)") (TriggeredSeconds :type "Float (double-precision)") (InputAction :type "InputAction Object Reference" :default "/Game/Blueprints/Inputs/IA_MoveRight.IA_MoveRight"))
  (:`Triggered`
    (set `self.OrientedDirection` (`KismetMathLibrary.MakeVector` (stale `EnhancedInput|/Game/Blueprints/Inputs/IA_MoveForward` ActionValue) ActionValue) :!label _label))
  (:`Canceled`
    (set `self.OrientedDirection` (0.0 0.0 0.0) :!label _label_2))
  (:`Completed`
    (goto _label_2)))

(event `EnhancedInput|/Game/Blueprints/Inputs/IA_MoveForward`
  (params (ActionValue :type "Float (double-precision)") (ElapsedSeconds :type "Float (double-precision)") (TriggeredSeconds :type "Float (double-precision)") (InputAction :type "InputAction Object Reference" :default "/Game/Blueprints/Inputs/IA_MoveForward.IA_MoveForward"))
  (:`Triggered`
    (goto _label))
  (:`Canceled`
    (goto _label_2))
  (:`Completed`
    (goto _label_2)))

(fn `Fire`
  (`|SpawnActorFromClass` "/Game/Blueprints/BP_Bullet.BP_Bullet_C" (`KismetMathLibrary.MakeTransform` (`SceneComponent.K2_GetComponentLocation` (`self.Muzzle`))) "AlwaysSpawn" "MultiplyWithRoot" null null)
  (set `self.CurrentFireDelay` 0.0))

(fn `Hit`
  (`self.K2_DestroyActor`))

(fn `Move`
  (params (DirectionVector :type "Vector Structure") (Speed :type "Float (double-precision)"))
  (locals (NewLocalVar :type "Float (double-precision)" :default 0.0))
  (`self.K2_SetActorLocation` (+ (* DirectionVector Speed (`GameplayStatics.GetWorldDeltaSeconds`)) (`self.K2_GetActorLocation`)) true))

(fn `UserConstructionScript`)